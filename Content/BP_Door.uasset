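; BP_Door is a door actor that swings open and shut when its OpenDoor event is called.
; Overlapping InteractionBox registers the door as CurrentDoor on BP_FirstPersonCharacter, and leaving clears that reference.
; OpenDoor flips IsOpen and snaps the DoorPrivot component between closed and a 90-degree relative rotation, with no animation.
; CanInteract is reset on any end overlap but is never set true or read here.
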(event OnComponentBeginOverlap(InteractionBox)
  (params (OverlappedComponent :type Primitive%20Component%20Object%20Reference) (OtherActor :type Actor%20Object%20Reference) (OtherComp :type Primitive%20Component%20Object%20Reference) (OtherBodyIndex :type Integer) (bFromSweep :type Boolean) (SweepResult :type Hit%20Result%20Structure%20%28by%20ref%29))
  (bind _asbp_first_person_character (Utilities|Casting|CastToBP_FirstPersonCharacter OtherActor))
  (Variables|/Game/FirstPerson/Blueprints/BP_FirstPersonCharacter.BP_FirstPersonCharacter_C|SetCurrentDoor _asbp_first_person_character self))

(event OnComponentEndOverlap(InteractionBox)
  (params (OverlappedComponent :type Primitive%20Component%20Object%20Reference) (OtherActor :type Actor%20Object%20Reference) (OtherComp :type Primitive%20Component%20Object%20Reference) (OtherBodyIndex :type Integer))
  (Variables|Default|SetCanInteract false)
  (bind _asbp_first_person_character (Utilities|Casting|CastToBP_FirstPersonCharacter OtherActor))
  (Variables|/Game/FirstPerson/Blueprints/BP_FirstPersonCharacter.BP_FirstPersonCharacter_C|SetCurrentDoor _asbp_first_person_character 0))

(event Custom|OpenDoor
  (if (Variables|Default|GetIsOpen)
    (Transformation|SetRelativeRotation (Variables|Default|GetDoorPrivot) "0, 0, 0" false false)
    (Variables|Default|SetIsOpen false)
    (else
      (Transformation|SetRelativeRotation (Variables|Default|GetDoorPrivot) "0.000000,90.000000,0.000000" false false)
      (Variables|Default|SetIsOpen true))))

(event EventBeginPlay)

(event Collision|EventActorBeginOverlap
  (params (OtherActor :type Actor%20Object%20Reference)))

(event EventTick
  (params (DeltaSeconds :type Float%20%28single-precision%29)))

(fn ConstructionScript)